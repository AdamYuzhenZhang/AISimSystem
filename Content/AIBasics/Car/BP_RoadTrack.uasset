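; BP_RoadTrack is a road actor that spawns randomized two-way traffic as BP_CarSimulator actors.
; Each Tick, enabled directions roll car density times delta time against a random number, approximating a spawn rate per second.
; Cars spawn far below the world, then receive the track reference and a random lane offset.
; Forward lanes use positive indices; backward lanes use zero or negative ones and flag opposite direction.
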(event `self.ReceiveTick`
  (params (DeltaSeconds :type "Float (single-precision)"))
  (`|ExecutionSequence`
    (:`then_0`
      (if (`self.IsForward`)
        (`self.ForwardGeneration` DeltaSeconds)))
    (:`then_1`
      (if (`self.IsBackward`)
        (`self.BackwardGeneration` DeltaSeconds)))))

(event `ForwardGeneration`
  (params (DeltaS :type "Float (double-precision)"))
  (if (> (* DeltaS (`self.ForwardCarDensity`)) (`KismetMathLibrary.RandomFloatInRange` 0.0 1.0))
    (bind _returnvalue (`|SpawnActorFromClass` "/AISimSystem/AIBasics/Car/BP_CarSimulator.BP_CarSimulator_C" (`KismetMathLibrary.MakeTransform` (0.0 0.0 -100000000.0)) "AdjustIfPossibleButAlwaysSpawn" "OverrideRootScale" null null))
    (set `/AISimSystem/AIBasics/Car/BP_CarSimulator.RoadTrack` self _returnvalue)
    (`/AISimSystem/AIBasics/Car/BP_CarSimulator.SetOffSet` _returnvalue (`KismetMathLibrary.RandomIntegerInRange` 1 (`self.FowardRoadLaneNum`)))))

(event `BackwardGeneration`
  (params (DeltaS :type "Float (double-precision)"))
  (if (> (* DeltaS (`self.BackwardCarDensity`)) (`KismetMathLibrary.RandomFloatInRange` 0.0 1.0))
    (bind _returnvalue (`|SpawnActorFromClass` "/AISimSystem/AIBasics/Car/BP_CarSimulator.BP_CarSimulator_C" (`KismetMathLibrary.MakeTransform` (0.0 0.0 -100000000.0)) "AdjustIfPossibleButAlwaysSpawn" "OverrideRootScale" null null))
    (set `/AISimSystem/AIBasics/Car/BP_CarSimulator.RoadTrack` self _returnvalue)
    (`/AISimSystem/AIBasics/Car/BP_CarSimulator.SetOffSet` _returnvalue (`KismetMathLibrary.RandomIntegerInRange` 0 (- 1 (`self.BackwardRoadlaneNum`))))
    (set `/AISimSystem/AIBasics/Car/BP_CarSimulator.OppositeDirection` true _returnvalue)))

(fn `UserConstructionScript`)