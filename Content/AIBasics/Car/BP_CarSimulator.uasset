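; BP_CarSimulator is a car actor that drives along its RoadTrack's spline in either direction and destroys itself at the end.
; Forward and backward timelines drive distance along the spline, shifting position sideways by a lane offset computed in SetOffSet.
; Timeline play rate is speed divided by spline length, keeping speed independent of road length.
; SlowDown and SpeedUp events use further timelines to scale that rate over time.
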(event `self.ReceiveBeginPlay`
  (`KismetSystemLibrary.Delay` 0.2)
  (if (`self.OppositeDirection`)
    (`self.MoveCarBackward`)
    (else
      (`self.MoveCarForward`))))

(event `MoveCarForward`
  (bind _roadspline (`/AISimSystem/AIBasics/Car/BP_RoadTrack.RoadSpline` (`self.RoadTrack`)))
  (`self.SetPlayRate`)
  (bind (_direction _movement_track) (`Timeline|CarMovement`)
    (:`Update`
      (bind _returnvalue (`KismetMathLibrary.Lerp` 0.0 (`SplineComponent.GetSplineLength` _roadspline) _movement_track))
      (bind _returnvalue_2 (`SplineComponent.GetRotationAtDistanceAlongSpline` _roadspline _returnvalue "World"))
      (`self.K2_SetActorLocationAndRotation` (+ (`SplineComponent.GetLocationAtDistanceAlongSpline` _roadspline _returnvalue "World") (* (`KismetMathLibrary.GetRightVector` _returnvalue_2) (`self.OffSet`))) _returnvalue_2))
    (:`Finished`
      (`self.K2_DestroyActor`))))

(event `MoveCarBackward`
  (bind _roadspline (`/AISimSystem/AIBasics/Car/BP_RoadTrack.RoadSpline` (`self.RoadTrack`)))
  (`self.SetPlayRate`)
  (bind (_direction _newtrack_0) (`Timeline|CarMovementBack`)
    (:`Update`
      (bind _returnvalue (`KismetMathLibrary.Lerp` (`SplineComponent.GetSplineLength` _roadspline) 0.0 _newtrack_0))
      (bind _returnvalue_2 (`SplineComponent.GetRotationAtDistanceAlongSpline` _roadspline _returnvalue "World"))
      (`self.K2_SetActorLocationAndRotation` (+ (`SplineComponent.GetLocationAtDistanceAlongSpline` _roadspline _returnvalue "World") (* (`KismetMathLibrary.GetRightVector` _returnvalue_2) (`self.OffSet`))) _returnvalue_2))
    (:`Finished`
      (`self.K2_DestroyActor`))))

(event `SlowDown`
  (bind (_direction _speedchange) (`Timeline|ChangeSpeedDown`)
    (:`Update`
      (`TimelineComponent.SetPlayRate` (`self.CarMovement`) (* _speedchange (`self.PlayRate`)))
      (`TimelineComponent.SetPlayRate` (`self.CarMovementBack`) (* _speedchange (`self.PlayRate`))))))

(event `SpeedUp`
  (bind (_direction _speedchange) (`Timeline|ChangeSpeedUp`)
    (:`Update`
      (`TimelineComponent.SetPlayRate` (`self.CarMovement`) (* _speedchange (`self.PlayRate`)))
      (`TimelineComponent.SetPlayRate` (`self.CarMovementBack`) (* _speedchange (`self.PlayRate`))))))

(fn `SetOffSet`
  (params (OffSetNum :type Integer))
  (set `self.OffSet` (- (* OffSetNum 350) 170)))

(fn `SetPlayRate`
  (bind _returnvalue (/ (`self.CurrentSpeed`) (`SplineComponent.GetSplineLength` (`/AISimSystem/AIBasics/Car/BP_RoadTrack.RoadSpline` (`self.RoadTrack`)))))
  (`TimelineComponent.SetPlayRate` (`self.CarMovement`) _returnvalue)
  (`TimelineComponent.SetPlayRate` (`self.CarMovementBack`) _returnvalue)
  (set `self.PlayRate` _returnvalue))

(fn `UserConstructionScript`)