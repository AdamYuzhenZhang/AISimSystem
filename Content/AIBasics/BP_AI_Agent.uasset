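; BP_AI_Agent is an AI agent that picks attractor locations to visit when it perceives them.
; Each tick it copies the current hour from BP_SunPosition.
; Perception updates while the blackboard task is Idle consider unvisited Locations tagged ATTRACTOR, filtered by a random roll against attraction level and by free capacity.
; A chosen Location gains an occupant and becomes SightseeingActor, and CurrentTask is set to IDLING.
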(event `self.ReceiveBeginPlay`
  (bind _outactors (`GameplayStatics.GetAllActorsOfClass` "/SunPosition/BP_SunPosition.BP_SunPosition_C"))
  (set `self.SunPos` (`|GetArrayItem` _outactors)))

(event `self.ReceiveTick`
  (params (DeltaSeconds :type "Float (single-precision)"))
  ;[1 1 1] Set Current Hour
  (set `self.CurrentHour` (`/SunPosition/BP_SunPosition.Hours` (`self.SunPos`))))

(event `self.PerceptionComponent.OnTargetPerceptionUpdated`
  (params (Actor :type "Actor Object Reference") (Stimulus :type "AIStimulus Structure"))
  ;[1 1 1] On Target Perception Updated
  (if (== (`BlackboardComponent.GetValueAsEnum` (`self.BlackboardComp`) (`self.BBCurrentTask`)) (`self.Idle`))
    (`self.FindInterestingPlaceToVisit` Actor)))

(event `FindInterestingPlaceToVisit`
  (params (UpdatedActors :type "Actor Object Reference"))
  ;[1 1 1] If see attractor, set it as target and change current task to sightseeing
  (if (`self.ActorHasTag` UpdatedActors "ATTRACTOR")
    (bind _aslocation (cast `Location` UpdatedActors))
    (if (`KismetArrayLibrary.Array_Contains` (`self.VisitedAttractor`) _aslocation)
      _
      (elif (< (`KismetMathLibrary.RandomIntegerInRange` 0 10) (`Location.AttractionLevel` _aslocation))
        (bind _currentnumber (`Location.CurrentNumber` _aslocation))
        (if (> (`Location.Capacity` _aslocation) _currentnumber)
          (set `Location.CurrentNumber` (+ _currentnumber 1) _aslocation)
          (set `self.SightseeingActor` _aslocation)
          (set `self.CurrentTask` "IDLING"))))))

(fn `UserConstructionScript`)