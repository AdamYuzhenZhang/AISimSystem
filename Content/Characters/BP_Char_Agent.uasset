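; BP_Char_Agent is an AI agent character with a selection indicator, toggleable floating text and debug path display.
; Selection and text functions switch component visibility; while shown, Tick updates the text and turns it toward the player pawn.
; With DrawPath on, Tick recomputes a navmesh path to the RandomTargetInRange blackboard location using NavQueryFilter_Pedestrian and draws it as debug lines.
; A spline-mesh drawing alternative is left unconnected.
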(event `self.ReceiveTick`
  (params (DeltaSeconds :type "Float (single-precision)"))
  (bind _charactertext (`self.CharacterText`))
  (`|ExecutionSequence`
    (:`then_0`
      ;[1 1 1] Set Character Text and Face Player
      (if (`self.CharTextVisible`)
        (`TextRenderComponent.K2_SetText` _charactertext (`self.CharText`))
        (`SceneComponent.K2_SetWorldRotation` _charactertext (`KismetMathLibrary.MakeRotFromX` (- (`self.K2_GetActorLocation` (`GameplayStatics.GetPlayerPawn` 0)) (`SceneComponent.K2_GetComponentLocation` _charactertext))) false false)))
    (:`then_1`
      (if (`self.DrawPath`)
        (`self.DrawNavPath`)))))

(fn `DeselectChar`
  (`SceneComponent.SetVisibility` (`self.SelectionIndicator`) false false))

(fn `DrawNavPath`
  (bind _returnvalue (`NavigationSystemV1.FindPathToLocationSynchronously` (`self.K2_GetActorLocation`) (`BlackboardComponent.GetValueAsVector` (`AIBlueprintHelperLibrary.GetBlackboard` null) "RandomTargetInRange") null "/AISimSystem/AIBasics/Navigation/NavQueryFilters/NavQueryFilter_Pedestrian.NavQueryFilter_Pedestrian_C"))
  (bind _pathpoints (`NavigationPath.PathPoints` _returnvalue))
  (for _index (range (+ (- (`KismetArrayLibrary.Array_Length` _pathpoints) 2) 1))
    (`KismetSystemLibrary.DrawDebugLine` (`|GetArrayItem` _pathpoints _index) (`|GetArrayItem` _pathpoints (+ _index 1)) (struct :`G` 0.032141 :`B` 1.0 :`A` 1.0) 0.0 10.0)))

(fn `SelectChar`
  (`SceneComponent.SetVisibility` (`self.SelectionIndicator`) true false))

(fn `ToggleCharTextVisible`
  (bind _charactertext (`self.CharacterText`))
  (if (`self.CharTextVisible`)
    (set `self.CharTextVisible` false)
    (`SceneComponent.SetVisibility` _charactertext false false)
    (else
      (set `self.CharTextVisible` true)
      (`SceneComponent.SetVisibility` _charactertext true false))))

(fn `UserConstructionScript`)