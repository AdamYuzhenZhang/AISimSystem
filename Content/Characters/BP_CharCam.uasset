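; BP_CharCam is a scene-capture camera actor that follows a target character with top, third-person and first-person views.
; FollowChar snaps and attaches it to the target, enables per-frame capture and prints both transforms for debugging.
; DisableCam detaches it and stops per-frame capture.
; The three view functions switch framing by setting the SpringArm's length and relative rotation.
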(fn `DisableCam`
  (`self.K2_DetachFromActor` "KeepRelative")
  (set `SceneCaptureComponent.bCaptureEveryFrame` false (`self.SceneCaptureComponent2D`)))

(fn `FollowChar`
  (params (TargetChar :type "/AISimSystem/Characters/BP_Char_Agent Object Reference"))
  (`self.K2_SetActorTransform` (`self.GetTransform` TargetChar))
  (`self.K2_AttachToActor` TargetChar "None" "SnapToTarget" "SnapToTarget" "SnapToTarget" false)
  (set `SceneCaptureComponent.bCaptureEveryFrame` true (`self.SceneCaptureComponent2D`))
  (`KismetSystemLibrary.PrintString` "CameraTransform" true true (struct :`R` 1.0 :`B` 0.004547 :`A` 1.0))
  (`KismetSystemLibrary.PrintString` (`KismetStringLibrary.Conv_TransformToString` (`self.GetTransform`)) true true (struct :`R` 1.0 :`G` 0.017466 :`A` 1.0))
  (`KismetSystemLibrary.PrintString` "CharCurrentTransform" true true (struct :`R` 0.895106 :`B` 1.0 :`A` 1.0))
  (`KismetSystemLibrary.PrintString` (`KismetStringLibrary.Conv_TransformToString` (`self.GetTransform` TargetChar)) true true (struct :`R` 1.0 :`B` 0.953341 :`A` 1.0)))

(fn `SetFirstPerson`
  (bind _springarm (`self.SpringArm`))
  (set `SpringArmComponent.TargetArmLength` 0.0 _springarm)
  (`SceneComponent.K2_SetRelativeTransform` _springarm (`KismetMathLibrary.MakeTransform` (0.0 0.0 0.0)) false false))

(fn `SetThirdPerson`
  (bind _springarm (`self.SpringArm`))
  (set `SpringArmComponent.TargetArmLength` 300.0 _springarm)
  (`SceneComponent.K2_SetRelativeTransform` _springarm (`KismetMathLibrary.MakeTransform` (0.0 0.0 0.0)) false false))

(fn `SetTopView`
  (bind _springarm (`self.SpringArm`))
  (set `SpringArmComponent.TargetArmLength` 300.0 _springarm)
  (`SceneComponent.K2_SetRelativeTransform` _springarm (`KismetMathLibrary.MakeTransform` (0.0 0.0 0.0) (struct :`Pitch` -90.0)) false false))

(fn `UserConstructionScript`)