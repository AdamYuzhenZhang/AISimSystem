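; AI simulation volume with an orthographic scene-capture camera that lets screen positions pick agents or world points within it.
; On BeginPlay it sizes the capture width and spring arm from the sphere volume's scale and optionally creates the UMG_AISim widget.
; A 2D ratio becomes an offset on the camera plane for a forward line trace with debug drawing.
; Hits select a BP_Char_Agent or spawn a TestActor, or return the location.
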(event `self.ReceiveBeginPlay`
  (bind _returnvalue (`KismetMathLibrary.GetMaxElement` (`SceneComponent.K2_GetComponentScale` (`self.SphereVolume`))))
  (bind _output_get (set `SceneCaptureComponent2D.OrthoWidth` (* 72 _returnvalue) (`self.SceneCaptureComponent2D`)))
  (set `self.BoundingValue` _output_get)
  (set `SpringArmComponent.TargetArmLength` (* 30 _returnvalue) (`self.SpringArm`))
  (if (`self.AutoSpawnUMG`)
    (bind _returnvalue_2 (`|CreateWidget` "/AISimSystem/AI_UMG/UMG_AISim.UMG_AISim_C" (`GameplayStatics.GetPlayerController` 0)))
    (`UserWidget.AddToViewport` _returnvalue_2 0)))

(fn `LineTracing`
  (params (XYRatio :type "Vector2D Structure"))
  (returns (HitResult :type "HitResult Structure") (ReturnValue :type Boolean))
  (bind (_x _y) (`KismetMathLibrary.BreakVector2D` XYRatio))
  (bind _scenecapturecomponent2d (`self.SceneCaptureComponent2D`))
  (bind _returnvalue (+ (`SceneComponent.K2_GetComponentLocation` _scenecapturecomponent2d) (`KismetMathLibrary.GreaterGreater_VectorRotator` (* (`KismetMathLibrary.MakeVector` 0.0 _x _y) (`SceneCaptureComponent2D.OrthoWidth` _scenecapturecomponent2d)) (`SceneComponent.K2_GetComponentRotation` _scenecapturecomponent2d))))
  (bind _returnvalue_2 (+ _returnvalue (* (`SceneComponent.GetForwardVector` _scenecapturecomponent2d) 10000)))
  (bind (_outhit _returnvalue_3) (`KismetSystemLibrary.LineTraceSingle` _returnvalue _returnvalue_2 "TraceTypeQuery1"))
  (`KismetSystemLibrary.DrawDebugLine` _returnvalue _returnvalue_2 (struct :`R` 1.0 :`B` 0.670939 :`A` 1.0) 1.0 5.0)
  (return _outhit _returnvalue_3))

(fn `SelectThroughCamera`
  (params (XYRatio :type "Vector2D Structure"))
  (returns (SelectedChar :type "/AISimSystem/Characters/BP_Char_Agent Object Reference"))
  (bind (_hitresult _returnvalue) (`self.LineTracing` XYRatio))
  (if _returnvalue
    (bind (_bblockinghit _binitialoverlap _time _distance _location _impactpoint _normal _impactnormal _physmat _hitactor) (`GameplayStatics.BreakHitResult` _hitresult))
    (bind _asbp_char_agent (cast `/AISimSystem/Characters/BP_Char_Agent` _hitactor)
      (:`then`
        (`/AISimSystem/Characters/BP_Char_Agent.SelectChar` _asbp_char_agent)
        (return _asbp_char_agent))
      (:`CastFailed`
        (`|SpawnActorFromClass` "/AISimSystem/AI_UMG/TestActor.TestActor_C" (`KismetMathLibrary.MakeTransform` _location) "Undefined" "OverrideRootScale" null null)
        (return null)))))

(fn `UserConstructionScript`)

(fn `WorldLocationThroughCamera`
  (params (XYRatio :type "Vector2D Structure"))
  (returns (SelectedLocation :type "Vector Structure"))
  (bind (_hitresult _returnvalue) (`self.LineTracing` XYRatio))
  (if _returnvalue
    (return (`.Location` (`GameplayStatics.BreakHitResult` _hitresult)))))